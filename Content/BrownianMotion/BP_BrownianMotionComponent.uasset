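; Actor component that makes its owning actor drift around its starting position with smooth Brownian-style motion.
; BeginPlay caches the root component's relative location as the origin.
; While motion is enabled, each Tick samples 1D Perlin noise per axis, using staggered time offsets to decorrelate them.
; The result, shaped by frequency, scale and amplitude, is added to the origin and position offset without sweeping.
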(event EventBeginPlay
  (Variables|BrownianMotion|SetStartingPosition (Variables|/Script/Engine.SceneComponent|GetRelativeLocation (Variables|/Script/Engine.Actor|GetRootComponent (Components|GetOwner)))))

(event EventTick
  (params (DeltaSeconds :type Float%20%28single-precision%29))
  (bind _returnvalue (Utilities|Time|GetGameTimeinSeconds))
  (bind _timeoffset (Variables|BrownianMotion|GetTimeOffset))
  (if (Variables|BrownianMotion|GetbEnableMotion)
    (Transformation|SetActorRelativeLocation (Components|GetOwner) (+ (Variables|BrownianMotion|GetStartingPosition) (Variables|BrownianMotion|GetPositionOffset) (* (Math|Vector|MakeVector (Class|KismetMathLibrary|PerlinNoise1D (* (+ _returnvalue _timeoffset) (Variables|BrownianMotion|GetFrequency))) (Class|KismetMathLibrary|PerlinNoise1D (* (+ _returnvalue 1e+01 _timeoffset) (Variables|BrownianMotion|GetFrequency))) (Class|KismetMathLibrary|PerlinNoise1D (* (+ _returnvalue 3e+01 _timeoffset) (Variables|BrownianMotion|GetFrequency)))) (Variables|BrownianMotion|GetScale) (Variables|BrownianMotion|GetAmplitude))))))