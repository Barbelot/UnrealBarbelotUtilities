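; Audio analysis actor that turns pre-baked NRT onset and loudness data into live per-channel onset and loudness values.
; Time comes from its audio component's playback percent, or from a Sequencer player when audio playback is off.
; Left and right onsets average strengths over a time window, rise at a capped rate, decay on Tick, and blend into a scaled mean.
; Optional debug spheres scale with each value.
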(event Custom|OnAudioPlayback
  (params (PlayingSoundWave :type Sound%20Wave%20Object%20Reference) (PlaybackPercent :type Float%20%28single-precision%29))
  (bind _soundduration (Variables|BAAudioAnalysis|GetSoundDuration))
  (bind _returnvalue (* PlaybackPercent _soundduration))
  (CallFunction|UpdateOnset _returnvalue 0.016667)
  (CallFunction|UpdateLoudness _returnvalue))

(event EventBeginPlay
  (if (Variables|BAAudioAnalysis|GetPlayAudio)
    (EventDispatchers|BindEventtoOnAudioPlaybackPercent (Variables|Components|GetAudio) (delegate Custom|OnAudioPlayback)))
  (CallFunction|UpdateDebug)
  (if (Variables|BAAudioAnalysis|GetPlayAudio)
    (Audio|Components|Audio|Play (Variables|Components|GetAudio) 0.0)
    (else
      (Audio|Components|Audio|Stop (Variables|Components|GetAudio)))))

(event EventTick
  (params (DeltaSeconds :type Float%20%28single-precision%29))
  (bind _onsetfalloffspeed (Variables|BAAudioAnalysis|Onset|GetOnsetFalloffSpeed))
  (bind _sequencetimeoffset (Variables|BAAudioAnalysis|GetSequenceTimeOffset))
  (bind _sequence (Variables|BAAudioAnalysis|GetSequence))
  (bind _returnvalue (* DeltaSeconds _onsetfalloffspeed))
  (bind _sequenceplayer (Variables|/Script/LevelSequence.LevelSequenceActor|GetSequencePlayer _sequence))
  (bind _returnvalue_2 (Sequencer|Player|GetCurrentTime _sequenceplayer))
  (bind (_frame _framerate) (Utilities|TimeManagement|BreakQualifiedFrameTime _returnvalue_2))
  (bind _value (Utilities|Struct|BreakFrameNumber _frame))
  (bind (_numerator _denominator) (Class|KismetMathLibrary|BreakFrameRate _framerate))
  (bind _returnvalue_3 (Math|Conversions|ToFloat(Integer) _numerator))
  (bind _returnvalue_4 (/ _returnvalue_3 _denominator))
  (bind _returnvalue_5 (/ _value _returnvalue_4))
  (bind _returnvalue_6 (+ _returnvalue_5 _sequencetimeoffset))
  ;[1 1 1] Update Falloff
  (Variables|BAAudioAnalysis|Onset|SetCurrentOnsetLeft (Math|Float|Max(Float) 0.0 (- (Variables|BAAudioAnalysis|Onset|GetCurrentOnsetLeft) _returnvalue)))
  (Variables|BAAudioAnalysis|Onset|SetCurrentOnsetRight (Math|Float|Max(Float) 0.0 (- (Variables|BAAudioAnalysis|Onset|GetCurrentOnsetRight) _returnvalue)))
  (Utilities|FlowControl|Sequence
    (:then_0
      (if (not (Variables|BAAudioAnalysis|GetPlayAudio))
        (CallFunction|UpdateOnset _returnvalue_6 DeltaSeconds)
        (CallFunction|UpdateLoudness _returnvalue_6)))
    (:then_1
      ;[1 1 1] Update Debug Spheres
      (if (Variables|BAAudioAnalysis|GetShowDebugSphere)
        (Transformation|SetRelativeScale3D (Variables|Default|GetOnsetRight) (Math|Conversions|ToVector(Float) (Variables|BAAudioAnalysis|Onset|GetCurrentOnsetRight)))
        (Transformation|SetRelativeScale3D (Variables|Default|GetOnsetLeft) (Math|Conversions|ToVector(Float) (Variables|BAAudioAnalysis|Onset|GetCurrentOnsetLeft)))))))

(fn ConstructionScript
  (bind _loudnessnrt (Variables|BAAudioAnalysis|Loudness|GetLoudnessNRT))
  (bind _sound (Variables|/Script/AudioAnalyzer.AudioAnalyzerNRT|GetSound _loudnessnrt))
  (Audio|Components|Audio|SetSound (Variables|Components|GetAudio) _sound)
  (Variables|BAAudioAnalysis|SetSoundDuration (Variables|/Script/Engine.SoundBase|GetDuration _sound))
  (CallFunction|UpdateDebug))

(fn UpdateOnset
  (params (Time :type Float%20%28double-precision%29) (DeltaTime :type Float%20%28double-precision%29))
  (bind _onsetnrt (Variables|BAAudioAnalysis|Onset|GetOnsetNRT))
  (bind _onsetnrt_2 (Variables|BAAudioAnalysis|Onset|GetOnsetNRT))
  (bind _onsettimewindow (Variables|BAAudioAnalysis|Onset|GetOnsetTimeWindow))
  (bind _onsettimewindow_2 (Variables|BAAudioAnalysis|Onset|GetOnsetTimeWindow))
  (bind _onsettimeoffset (Variables|BAAudioAnalysis|Onset|GetOnsetTimeOffset))
  (bind _returnvalue (+ Time _onsettimeoffset))
  (bind _returnvalue_2 (- _returnvalue _onsettimewindow_2))
  (bind _returnvalue_3 (- _returnvalue _onsettimewindow))
  (bind _outonsetstrengths (Class|OnsetNRT|GetNormalizedChannelOnsetsBetweenTimes _onsetnrt _returnvalue_2 _returnvalue 1))
  (bind _outonsetstrengths_2 (Class|OnsetNRT|GetNormalizedChannelOnsetsBetweenTimes _onsetnrt_2 _returnvalue_3 _returnvalue))
  (bind _returnvalue_4 (Utilities|Array|Length _outonsetstrengths))
  (bind _returnvalue_5 (Utilities|Array|Length _outonsetstrengths_2))
  (Utilities|FlowControl|Sequence
    (:then_0
      ;[0 0 0] LeftOnset
      (if (> _returnvalue_5 0)
        (for _array_element _outonsetstrengths_2
          (LocalVariables|SetOnsetSum (+ _array_element (LocalVariables|GetOnsetSum))))
        (if (> (/ (LocalVariables|GetOnsetSum) _returnvalue_5) (Variables|BAAudioAnalysis|Onset|GetCurrentOnsetLeft))
          (Variables|BAAudioAnalysis|Onset|SetCurrentOnsetLeft (Math|Float|Min(Float) (/ (LocalVariables|GetOnsetSum) _returnvalue_5) (+ (Variables|BAAudioAnalysis|Onset|GetCurrentOnsetLeft) (* DeltaTime (Variables|BAAudioAnalysis|Onset|GetOnsetRiseSpeed))))))))
    (:then_1
      (LocalVariables|SetOnsetSum 0.0))
    (:then_2
      ;[0 0 0] RightOnset
      (if (> _returnvalue_4 0)
        (for _array_element_2 _outonsetstrengths
          (LocalVariables|SetOnsetSum (+ _array_element_2 (LocalVariables|GetOnsetSum))))
        (if (> (/ (LocalVariables|GetOnsetSum) _returnvalue_4) (Variables|BAAudioAnalysis|Onset|GetCurrentOnsetRight))
          (Variables|BAAudioAnalysis|Onset|SetCurrentOnsetRight (Math|Float|Min(Float) (/ (LocalVariables|GetOnsetSum) _returnvalue_4) (+ (Variables|BAAudioAnalysis|Onset|GetCurrentOnsetRight) (* DeltaTime (Variables|BAAudioAnalysis|Onset|GetOnsetRiseSpeed))))))))
    (:then_3
      ;[0 0 0] Mean Onset
      (Variables|BAAudioAnalysis|Onset|SetCurrentOnset (* (+ (Variables|BAAudioAnalysis|Onset|GetCurrentOnsetLeft) (Variables|BAAudioAnalysis|Onset|GetCurrentOnsetRight)) 0.5 (Variables|BAAudioAnalysis|Onset|GetOnsetMultiplier))))))

(fn UpdateDebug
  (Rendering|SetVisibility (Variables|Default|GetOnsetRight) (Variables|BAAudioAnalysis|GetShowDebugSphere) true)
  (Rendering|SetVisibility (Variables|Default|GetOnsetLeft) (Variables|BAAudioAnalysis|GetShowDebugSphere) true)
  (Rendering|SetVisibility (Variables|Default|GetLoudness) (Variables|BAAudioAnalysis|GetShowDebugSphere) true))

(fn UpdateLoudness
  (params (Time :type Float%20%28single-precision%29))
  (Variables|BAAudioAnalysis|Loudness|SetCurrentLoudness (Class|LoudnessNRT|GetNormalizedLoudnessatTime (Variables|BAAudioAnalysis|Loudness|GetLoudnessNRT) Time))
  (if (Variables|BAAudioAnalysis|GetShowDebugSphere)
    (Transformation|SetRelativeScale3D (Variables|Default|GetLoudness) (Math|Conversions|ToVector(Float) (Variables|BAAudioAnalysis|Loudness|GetCurrentLoudness)))))